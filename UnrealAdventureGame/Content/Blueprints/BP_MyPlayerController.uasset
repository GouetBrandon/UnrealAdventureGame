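; BP_MyPlayerController is a player controller that holds HP and Mana and drives the life bar on the HUD.
; On BeginPlay it resets both stats to their maximums, then creates WBP_MyUI and adds it to the viewport.
; Pressing E calls ChangeHP with a fixed damage value, which sends clamped HP plus that change to the life bar without storing the result in HP.
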(event `self.ReceiveBeginPlay`
  (set `self.HP` (`self.HPMax`))
  (set `self.Mana` (`self.ManaMax`))
  (bind _returnvalue (`|CreateWidget` "/Game/Blueprints/WBP_MyUI.WBP_MyUI_C"))
  (bind _output_get (set `self.UI` _returnvalue))
  (`UserWidget.AddToViewport` _output_get 0))

(event `Key|E`
  (params (Key :type "Key Structure"))
  (:`Pressed`
    (`self.ChangeHP` -5.0)))

(fn `ChangeHP`
  (params (HPValue :type "Float (double-precision)"))
  (`/Game/Blueprints/WBP_MyUI.Set LifeBar` (`self.UI`) (+ (`KismetMathLibrary.FClamp` (`self.HP`) 0.0 (`self.HPMax`)) HPValue)))

(fn `UserConstructionScript`)